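; BP_TriggerGoalSphere is a goal trigger that awards a point to its owning player's golfer when the game's ball enters it.
; On BeginPlay it caches the BP_GolfGameMode.
; On overlap it checks the actor against the game mode's BallReference, looks up the golfer in the Players array by OwningPlayer index and increments that golfer's Points.
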(event `self.ReceiveBeginPlay`
  (bind _asbp_golf_game_mode (cast `/Game/Blueprints/BP_GolfGameMode` (`GameplayStatics.GetGameMode`)))
  (set `self.As BP Golf Game Mode` _asbp_golf_game_mode))

(event `self.ReceiveActorBeginOverlap`
  (params (OtherActor :type "Actor Object Reference"))
  (if (== OtherActor (`/Game/Blueprints/BP_GolfGameMode.BallReference` (`self.As BP Golf Game Mode`)))
    (bind _asbp_golfer (cast `/Game/Blueprints/BP_Golfer` (`|GetArrayItem` (`/Game/Blueprints/BP_GolfGameMode.Players` (`self.As BP Golf Game Mode`)) (`self.OwningPlayer`))))
    (`/Engine/EditorBlueprintResources/StandardMacros.IncrementInt` (`/Game/Blueprints/BP_Golfer.Points` _asbp_golfer))))

(fn `UserConstructionScript`)