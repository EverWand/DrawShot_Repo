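; Golf ball actor that registers with BP_GolfGameMode and reports which of four players reaches it once it stops rolling.
; In aim mode it disables physics and shows an arrow rotated by input, which grows on Tick after a delay.
; The arrow's scale sets hit strength, and reaching maximum notifies the game mode of a hit.
; HitBall re-enables physics and launches the ball along the arrow with an impulse.
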(event `self.ReceiveBeginPlay`
  ;[1 1 1] Begin Play
  (bind _asbp_golf_game_mode (cast `/Game/Blueprints/BP_GolfGameMode` (`GameplayStatics.GetGameMode`)))
  (bind _output_get (set `self.Golf Game Mode` _asbp_golf_game_mode))
  (`/Game/Blueprints/BP_GolfGameMode.RegisterBall` _output_get self) ; Register self with game mode
  (`SceneComponent.SetVisibility` (`self.Arrow`) false true) ; Hide Arrow and Club
)

(event `self.ReceiveActorBeginOverlap`
  (params (OtherActor :type "Actor Object Reference"))
  ;[1 1 1] Player Olverlap Ball
  (if (and (not (`self.IsRolling`)) (`self.BallRoaming`))
    (bind _playerindex (`self.CheckPlayerNumber` OtherActor)) ; Check which player overlapped - will not return if is not player
    (`/Game/Blueprints/BP_GolfGameMode.EventBallReached` (`self.Golf Game Mode`) _playerindex)
    (set `self.BallRoaming` false)))

(event `BallHitMode`
  (bind _arrow (`self.Arrow`))
  ;[1 1 1] Initialize Aim Mode
  (`SceneComponent.K2_SetWorldRotation` :`self` (`self.Sphere`)) ; Reset rotation
  (`SceneComponent.SetVisibility` _arrow true true) ; show arrow
  (`SceneComponent.SetRelativeScale3D` _arrow (0.0 0.0 0.0)) ; Set Arrow scale to 0
  (`PrimitiveComponent.SetSimulatePhysics` (`self.Sphere`) false) ; disable physics (because edge cases)
)

(event `HitBall`
  (bind _sphere (`self.Sphere`))
  ;[1 1 1] Hit Ball
  (`PrimitiveComponent.SetSimulatePhysics` _sphere true) ; Enable physics
  (`PrimitiveComponent.AddImpulse` _sphere (* (`KismetMathLibrary.GetForwardVector` (`SceneComponent.K2_GetComponentRotation` (`self.Arrow`))) (`self.HitStrength`) (`self.HitMultiplier`)) "None" true) ; launch in direction of arrow
  (`SceneComponent.SetVisibility` (`self.Arrow`) false true) ; Hide arrow and club
  (`SceneComponent.SetRelativeScale3D` (`self.Arrow`) (5.0 5.0 5.0)) ; Reset arrow scale
  (set `self.BallRoaming` true)
  (set `self.TotalDelta` 0.0) ; Reset time delay of for next shot
  (`GameplayStatics.PlaySound2D` "/Game/Audio/SFX/DrawShot_Sound_Library/Cymbal_Crash.Cymbal_Crash" 1.0 1.0 0.0 null null))

(event `SetAimRotation`
  (params (InputRotation :type "Vector2D Structure"))
  (bind (_x _y) (`KismetMathLibrary.BreakVector2D` InputRotation))
  ;[1 1 1] Aim Arrow rotation
  (if true
    (`SceneComponent.K2_SetRelativeRotation` (`self.Arrow`) (`KismetMathLibrary.FindLookAtRotation` (0.0 0.0 0.0) (`KismetMathLibrary.MakeVector` _y _x)) false false) ; Set rotation of arrow
  ))

(event `self.ReceiveTick`
  (params (DeltaSeconds :type "Float (single-precision)"))
  ;[1 1 1] Arrow Scale + delay
  (if (not (`self.BallRoaming`))
    (bind _output_get (set `self.TotalDelta` (+ DeltaSeconds (`self.TotalDelta`)))) ; Count delay
    (if (>= _output_get (`self.HitDelay`))
      (`self.ScaleArrow`) ; Scale from 0
    )))

(event `Reset Ball`
  (`self.K2_SetActorLocation` (1615.0 1725.0 20.0) false true)
  (`GameplayStatics.PlaySound2D` "/Game/Audio/SFX/DrawShot_Sound_Library/Hit_Additive_3.Hit_Additive_3" 1.0 1.0 0.0 null null))

(fn `CheckPlayerNumber`
  (params (ObjectOverlap :type "Object Object Reference"))
  (returns (PlayerIndex :type Integer))
  ;[1 1 1] Checks each player in sequence and only returns if overlapped is one of those players
  (if (== ObjectOverlap (`GameplayStatics.GetPlayerCharacter` 0))
    (return 0)
    (elif (== ObjectOverlap (`GameplayStatics.GetPlayerCharacter` 1))
      (return 1)
      (elif (== ObjectOverlap (`GameplayStatics.GetPlayerCharacter` 2))
        (return 2)
        (elif (== ObjectOverlap (`GameplayStatics.GetPlayerCharacter` 3))
          (return 3))))))

(fn `InputValidation`
  (params (InVec :type "Vector2D Structure"))
  (returns (WithinRange :type Boolean))
  (bind _inputdeadzone (`self.InputDeadzone`))
  (bind (_x _y) (`KismetMathLibrary.BreakVector2D` (`KismetMathLibrary.Normal2D` InVec)))
  (return (and (!= (`KismetMathLibrary.Abs` _x) 1.0) (> (`KismetMathLibrary.Abs` _x) _inputdeadzone) (!= (`KismetMathLibrary.Abs` _y) 1.0) (> (`KismetMathLibrary.Abs` _y) _inputdeadzone))))

(fn `IsRolling`
  (returns (IsRolling :type Boolean))
  (return (> (`KismetMathLibrary.VSize` (`SceneComponent.GetComponentVelocity` (`self.Sphere`))) (`self.StoppedRollingAcceptance`))))

(fn `ScaleArrow`
  (bind _arrow (`self.Arrow`))
  (bind _relativescale3d (`SceneComponent.RelativeScale3D` _arrow))
  (bind _x (.x _relativescale3d))
  (`SceneComponent.SetRelativeScale3D` _arrow (+ _relativescale3d (* (`GameplayStatics.GetWorldDeltaSeconds`) (`self.ScaleIncrement`)))) ; Scale Arrow
  (set `self.HitStrength` _x) ; Gets strength from scale of arrow
  (if (>= _x (`self.MaxHitStrength`))
    (`/Game/Blueprints/BP_GolfGameMode.EventBallHit` (`self.Golf Game Mode`))))

(fn `UserConstructionScript`)