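; BP_GolfGameMode is the game mode for a local multiplayer golf game, coordinating golfers and a shared ball.
; On BeginPlay it creates a local player per connected input device, numbers each BP_Golfer, then runs setup once all have spawned.
; The ball registers itself, then reach and hit events switch the current golfer and ball into hit mode, then return the golfer to roaming and launch the ball.
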(event `self.ReceiveBeginPlay`
  ;[1 1 1] Spawn and set up players
  (bind (_outinputdevices _returnvalue) (`InputDeviceLibrary.GetAllConnectedInputDevices`)) ; Count controllers
  (for _index (range _returnvalue)
    (`GameplayStatics.CreatePlayer` _index) ; Spawn player + controller
    (bind _asbp_golfer (cast `/Game/Blueprints/BP_Golfer` (`GameplayStatics.GetPlayerCharacter` _index)))
    (set `/Game/Blueprints/BP_Golfer.PlayerNumber` _index _asbp_golfer) ; Set player's number
    (`KismetArrayLibrary.Array_AddUnique` (`self.Players`) _asbp_golfer))
  (for _array_element (`self.Players`)
    (`/Game/Blueprints/BP_Golfer.SetupPlayer` _array_element) ; Allow players to set up after all spawned
  ))

(event `RegisterBall`
  (params (BallRef :type "/Game/Blueprints/BP_GolfBall Object Reference"))
  ;[1 1 1] Register ball for reference
  (set `self.BallReference` BallRef) ; Ball registering itself as a reference
)

(event `EventBallReached`
  (params (PlayerNumber :type Integer))
  ;[1 1 1] Get and cast to overlapped player
  (bind _asbp_golfer (cast `/Game/Blueprints/BP_Golfer` (`GameplayStatics.GetPlayerCharacter` PlayerNumber)))
  (bind _output_get (set `self.Current Golfer` _asbp_golfer))
  ;[1 1 1] Set Player and ball states
  (`/Game/Blueprints/BP_Golfer.PlayerHitMode` _output_get)
  (`/Game/Blueprints/BP_GolfBall.BallHitMode` (`self.BallReference`)))

(event `EventBallHit`
  ;[1 1 1] Reset player and launch ball
  (`/Game/Blueprints/BP_Golfer.PlayerRoamMode` (`self.Current Golfer`))
  (`/Game/Blueprints/BP_GolfBall.HitBall` (`self.BallReference`))
  (set `self.Current Golfer` null) ; Set value to null
)

(fn `UserConstructionScript`)