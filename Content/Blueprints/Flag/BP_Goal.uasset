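; BP_Goal is the golf goal flag that scores a point when the game's ball enters its ScoreArea.
; On BeginPlay it caches BP_GolfGameMode and applies the FlagColor material to its Cone mesh.
; An overlap matching the game mode's BallReference adds a point to the player's BP_Golfer, resets the ball and plays a 2D splat sound.
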(event `self.ReceiveBeginPlay`
  (`|ExecutionSequence`
    (:`then_0`
      (bind _asbp_golf_game_mode (cast `/Game/Blueprints/BP_GolfGameMode` (`GameplayStatics.GetGameMode`)))
      (set `self.Game Mode` _asbp_golf_game_mode))
    (:`then_1`
      (`PrimitiveComponent.SetMaterial` (`self.Cone`) 0 (`self.Flag Color`)))))

(event `self.ScoreArea.OnComponentBeginOverlap`
  (params (OverlappedComponent :type "PrimitiveComponent Object Reference") (OtherActor :type "Actor Object Reference") (OtherComp :type "PrimitiveComponent Object Reference") (OtherBodyIndex :type Integer) (bFromSweep :type Boolean) (SweepResult :type "HitResult Structure (by ref)"))
  (bind _ballreference (`/Game/Blueprints/BP_GolfGameMode.BallReference` (`self.Game Mode`)))
  (if (== OtherActor _ballreference)
    (bind _asbp_golfer (cast `/Game/Blueprints/BP_Golfer` (`GameplayStatics.GetPlayerCharacter` (`self.Player Index`))))
    (`/Game/Blueprints/BP_Golfer.Add Point` _asbp_golfer)
    (`/Game/Blueprints/BP_GolfBall.Reset Ball` _ballreference)
    (`GameplayStatics.PlaySound2D` "/Game/Audio/SFX/DrawShot_Sound_Library/Splat_Hit.Splat_Hit" 1.0 1.0 0.0 null null)))

(fn `UserConstructionScript`)